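; BP_Sword is a loot pickup that adds itself to the first-person character's inventory when overlapped.
; On BeginPlay it caches player 0 as BP_FirstPersonCharacter.
; On any overlap, without checking the other actor, it writes a self reference at InventoryIndex in that character's Inventory array and increments the index.
; It then destroys itself, so the stored reference points to a destroyed actor.
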(event EventBeginPlay
  (bind _asbp_first_person_character (Utilities|Casting|CastToBP_FirstPersonCharacter (Game|GetPlayerCharacter 0)))
  (Variables|Default|SetAs%20BP%20First%20Person%20Character _asbp_first_person_character))

(event Collision|EventActorBeginOverlap
  (params (OtherActor :type Actor%20Object%20Reference))
  (bind _as_bp_first_person_character (Variables|Default|GetAs%20BP%20First%20Person%20Character))
  (bind _as_bp_first_person_character_2 (Variables|Default|GetAs%20BP%20First%20Person%20Character))
  (if true
    (Utilities|Array|SetArrayElem (Variables|/Game/FirstPerson/Blueprints/BP_FirstPersonCharacter.BP_FirstPersonCharacter_C|GetInventory _as_bp_first_person_character) (Variables|/Game/FirstPerson/Blueprints/BP_FirstPersonCharacter.BP_FirstPersonCharacter_C|GetInventoryIndex _as_bp_first_person_character) self true)
    (Variables|/Game/FirstPerson/Blueprints/BP_FirstPersonCharacter.BP_FirstPersonCharacter_C|SetInventoryIndex _as_bp_first_person_character_2 (+ 1 (Variables|/Game/FirstPerson/Blueprints/BP_FirstPersonCharacter.BP_FirstPersonCharacter_C|GetInventoryIndex _as_bp_first_person_character_2)))
    (Actor|DestroyActor)))

(fn ConstructionScript
  (|CallParentFunction))